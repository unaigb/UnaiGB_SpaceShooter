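; Base space shooter power-up pickup whose PowerUpType selects heal, triple shot, time lapse, extra life or Ka Boom.
; The construction script tints the sphere per type through a dynamic material instance.
; Capsule overlap by BP_SS_Character disables collision, hides the sphere, applies the effect with a sound and destroys the actor.
; Ka Boom damages every BP_EnemyBase, with explosion, sound and self-destruction inside that loop.
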(event `self.Capsule.OnComponentBeginOverlap`
  (params (OverlappedComponent :type "PrimitiveComponent Object Reference") (OtherActor :type "Actor Object Reference") (OtherComp :type "PrimitiveComponent Object Reference") (OtherBodyIndex :type Integer) (bFromSweep :type Boolean) (SweepResult :type "HitResult Structure (by ref)"))
  (bind _asbp_ss_character (cast `/Game/SpaceShooter/Players/BP_SS_Character` OtherActor))
  (`self.SetActorEnableCollision` false)
  (`SceneComponent.SetHiddenInGame` (`self.Sphere`) true false)
  (switch `/Game/SpaceShooter/Power-Ups/PowerUpType` (`self.PowerUpType`)
    (:`NewEnumerator0`
      (`GameplayStatics.PlaySound2D` "/Game/SpaceShooter/Sounds/heal.heal" 1.0 1.0 0.0 null null)
      (set `/Game/SpaceShooter/Players/BP_SS_Character.HP` (`KismetMathLibrary.FClamp` (+ (`/Game/SpaceShooter/Players/BP_SS_Character.HP` _asbp_ss_character) 50.0) 0.0 100.0) _asbp_ss_character)
      (`self.K2_DestroyActor`))
    (:`NewEnumerator1`
      (`GameplayStatics.PlaySound2D` "/Game/SpaceShooter/Sounds/triple_shot.triple_shot" 1.0 1.0 0.0 null null)
      (`/Game/SpaceShooter/Players/BP_SS_Character.ActivateTripleShot` _asbp_ss_character)
      (`self.K2_DestroyActor`))
    (:`NewEnumerator2`
      (`GameplayStatics.PlaySound2D` "/Game/SpaceShooter/Sounds/time.time" 1.0 1.0 0.0 null null)
      (`/Game/SpaceShooter/Players/BP_SS_Character.ActivateTimeLapse` _asbp_ss_character)
      (`self.K2_DestroyActor`))
    (:`NewEnumerator3`
      (`GameplayStatics.PlaySound2D` "/Game/SpaceShooter/Sounds/1UP.1UP" 1.0 1.0 0.0 null null)
      (set `/Game/SpaceShooter/Players/BP_SS_Character.Lifes` (`KismetMathLibrary.Clamp` (+ (`/Game/SpaceShooter/Players/BP_SS_Character.Lifes` _asbp_ss_character) 1) 0 3) _asbp_ss_character)
      (`self.K2_DestroyActor`))
    (:`NewEnumerator4`
      (bind _outactors (`GameplayStatics.GetAllActorsOfClass` "/Game/SpaceShooter/Enemies/BP_EnemyBase.BP_EnemyBase_C"))
      (for _array_element _outactors
        (`GameplayStatics.ApplyDamage` _array_element 999.0)
        (`GameplayStatics.SpawnEmitterAtLocation` "/Game/StarterContent/Particles/P_Explosion.P_Explosion" (`self.K2_GetActorLocation`) (struct) (100.0 100.0 100.0))
        (`GameplayStatics.PlaySound2D` "/Game/SpaceShooter/Sounds/Kaboom_CoD_Sound_Effect.Kaboom_CoD_Sound_Effect" 1.0 1.0 0.0 null null)
        (`self.K2_DestroyActor`)))))

(fn `UserConstructionScript`
  (bind _returnvalue (`PrimitiveComponent.CreateDynamicMaterialInstance` (`self.Sphere`) 0 "/Game/SpaceShooter/Materials/M_LaserPointer-Outer.M_LaserPointer-Outer" "None"))
  (switch `/Game/SpaceShooter/Power-Ups/PowerUpType` (`self.PowerUpType`)
    (:`NewEnumerator0`
      (`MaterialInstanceDynamic.SetVectorParameterValue` _returnvalue "UserColor" (struct :`R` 0.152941 :`G` 0.615686 :`A` 1.0)))
    (:`NewEnumerator1`
      (`MaterialInstanceDynamic.SetVectorParameterValue` _returnvalue "UserColor" (struct :`R` 0.184123 :`B` 0.615686 :`A` 1.0)))
    (:`NewEnumerator2`
      (`MaterialInstanceDynamic.SetVectorParameterValue` _returnvalue "UserColor" (struct :`R` 0.033443 :`G` 0.222353 :`B` 0.615686 :`A` 1.0)))
    (:`NewEnumerator3`
      (`MaterialInstanceDynamic.SetVectorParameterValue` _returnvalue "UserColor" (struct :`R` 0.713542 :`G` 0.029731 :`B` 0.037598 :`A` 1.0)))
    (:`NewEnumerator4`
      (`MaterialInstanceDynamic.SetVectorParameterValue` _returnvalue "UserColor" (struct :`R` 0.615686 :`G` 0.282353 :`B` 0.070588 :`A` 1.0)))))