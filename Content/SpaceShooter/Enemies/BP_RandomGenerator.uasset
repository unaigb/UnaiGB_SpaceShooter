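; BP_RandomGenerator is the space shooter's enemy spawner, starting two seconds after BeginPlay.
; Its Spawn event re-calls itself after each game mode SpawnDelay to keep enemies coming.
; SpawnEnemy places enemies using randomly picked SpawnPoint-tagged components, offsetting BP_EnemyH on X.
; The class index depends on a Level 3 threshold, but its random ranges only yield zero, so BP_EnemyBase always spawns.
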(event `Spawn`
  (`self.SpawnEnemy`)
  (bind _asss_game_mode (cast `/Game/SpaceShooter/SS_GameMode` (`GameplayStatics.GetGameMode`)))
  (`/Engine/EditorBlueprintResources/StandardMacros.IsValid` _asss_game_mode
    (:`Is Valid`
      (`KismetSystemLibrary.Delay` (`/Game/SpaceShooter/SS_GameMode.SpawnDelay` _asss_game_mode))
      (`self.Spawn`))))

(event `self.ReceiveBeginPlay`
  (`KismetSystemLibrary.Delay` 2.0)
  (`self.Spawn`))

(event `self.ReceiveEndPlay`
  (params (EndPlayReason :type "EEndPlayReason Enum" :default "Destroyed")))

(fn `GetClassToSpawn`
  (params (Type :type Integer))
  (returns (ReturnValue :type "/Game/SpaceShooter/Enemies/BP_EnemyBase Class Reference"))
  (return (select `int` (`KismetMathLibrary.Clamp` Type 0 (- (`self.MaxNumEnemies`) 1)) :`0` "/Game/SpaceShooter/Enemies/BP_EnemyBase.BP_EnemyBase_C" :`1` "/Game/SpaceShooter/Enemies/BP_EnemyH.BP_EnemyH_C" :`2` "/Game/SpaceShooter/Enemies/BP_EnemyH.BP_EnemyH_C" :!type "/Game/SpaceShooter/Enemies/BP_EnemyBase Class Reference")))

(fn `SpawnEnemy`
  (returns (`Enemy Spawned` :type "/Game/SpaceShooter/Enemies/BP_EnemyBase Object Reference"))
  (bind _returnvalue (`self.GetComponentsByTag` "/Script/Engine.SceneComponent" "SpawnPoint"))
  (bind _location (.location (`SceneComponent.K2_GetComponentToWorld` (`|GetArrayItem` _returnvalue (`KismetMathLibrary.RandomInteger` (`KismetArrayLibrary.Array_Length` _returnvalue))))))
  (bind _asss_game_mode (cast `/Game/SpaceShooter/SS_GameMode` (`GameplayStatics.GetGameMode`)))
  (bind _returnvalue_2 (`self.GetClassToSpawn` (`KismetMathLibrary.RandomInteger` (select `bool` (>= (`/Game/SpaceShooter/SS_GameMode.Level` _asss_game_mode) 3) :`true` 1))))
  (bind _returnvalue_3 (`|SpawnActorFromClass` _returnvalue_2 (`KismetMathLibrary.MakeTransform` (select `bool` (== _returnvalue_2 "/Game/SpaceShooter/Enemies/BP_EnemyH.BP_EnemyH_C") :`false` _location :`true` (+ _location (-80.0 0.0 0.0))) (.rotation (`SceneComponent.K2_GetComponentToWorld` (`|GetArrayItem` _returnvalue (`KismetMathLibrary.RandomInteger` (`KismetArrayLibrary.Array_Length` _returnvalue))))) (.scale (`SceneComponent.K2_GetComponentToWorld` (`|GetArrayItem` _returnvalue (`KismetMathLibrary.RandomInteger` (`KismetArrayLibrary.Array_Length` _returnvalue)))))) "Undefined" "MultiplyWithRoot" null null))
  (return _returnvalue_3))

(fn `UserConstructionScript`)