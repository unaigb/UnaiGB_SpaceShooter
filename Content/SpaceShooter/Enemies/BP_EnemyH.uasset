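; BP_EnemyH is a space shooter enemy, a child Blueprint that starts with its movement vector set to its right vector.
; Overlapping a "Lateral" actor reverses that vector, drops the enemy along X and shortens its shot delay, with a low-end reset.
; Overlapping a "SupInf" actor subtracts score through SS_GameMode and destroys the enemy.
; Movement and shooting are not implemented here, only their variables are adjusted.
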(event `self.ReceiveBeginPlay`
  (`parent.ReceiveBeginPlay`)
  (set `self.MovementVector` (`self.GetActorRightVector`)))

(event `self.ReceiveActorBeginOverlap`
  (params (OtherActor :type "Actor Object Reference"))
  (bind _returnvalue (- (`self.DelayShoot`) 0.1))
  (`/Engine/EditorBlueprintResources/StandardMacros.IsValid` OtherActor
    (:`Is Valid`
      (`parent.ReceiveActorBeginOverlap` OtherActor)
      (if (`KismetArrayLibrary.Array_Contains` (`Actor.Tags` OtherActor) "Lateral")
        (set `self.MovementVector` (* (`self.MovementVector`) (-1.0 -1.0 -1.0)))
        (`self.K2_AddActorWorldOffset` (`KismetMathLibrary.MakeVector` (`self.Drop`)))
        (set `self.DelayShoot` _returnvalue)
        (if (< _returnvalue 0.0)
          (set `self.DelayShoot` 0.1))
        (elif (`KismetArrayLibrary.Array_Contains` (`Actor.Tags` OtherActor) "SupInf")
          (bind _asss_game_mode (cast `/Game/SpaceShooter/SS_GameMode` (`GameplayStatics.GetGameMode`)))
          (set `/Game/SpaceShooter/SS_GameMode.Score` (- (`/Game/SpaceShooter/SS_GameMode.Score` _asss_game_mode) 50) _asss_game_mode)
          (`self.K2_DestroyActor`))))))

(fn `UserConstructionScript`
  (`parent.UserConstructionScript`))