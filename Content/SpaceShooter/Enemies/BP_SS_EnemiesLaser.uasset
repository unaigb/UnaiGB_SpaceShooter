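; Enemy laser projectile for the space shooter that flies along its forward vector each Tick at Speed.
; Capsule overlap damages actors tagged Player and destroys the laser, which SupInf-tagged actors also destroy.
; A separate actor overlap with the player fires OnAmmoDestroy, explosion particles and sound, then a delayed destroy.
; On BeginPlay it lowers its own time dilation if the game mode's TiempoRalentizado slow-motion flag is set.
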(event `self.Capsule.OnComponentBeginOverlap`
  (params (OverlappedComponent :type "PrimitiveComponent Object Reference") (OtherActor :type "Actor Object Reference") (OtherComp :type "PrimitiveComponent Object Reference") (OtherBodyIndex :type Integer) (bFromSweep :type Boolean) (SweepResult :type "HitResult Structure (by ref)"))
  (`/Engine/EditorBlueprintResources/StandardMacros.IsValid` OtherActor
    (:`Is Valid`
      (if (`self.ActorHasTag` OtherActor "Player")
        (`GameplayStatics.ApplyDamage` OtherActor 20.0)
        (`self.K2_DestroyActor`)
        (elif (`self.ActorHasTag` OtherActor "SupInf")
          (`self.K2_DestroyActor`))))))

(event `self.ReceiveActorBeginOverlap`
  (params (OtherActor :type "Actor Object Reference"))
  (if (`KismetArrayLibrary.Array_Contains` (`Actor.Tags` OtherActor) "Player")
    (`self.OnAmmoDestroy`)
    (`GameplayStatics.SpawnEmitterAtLocation` "/Game/StarterContent/Particles/P_Explosion.P_Explosion" (`self.K2_GetActorLocation`))
    (`GameplayStatics.PlaySound2D` "/Game/StarterContent/Audio/Explosion02.Explosion02" 1.0 1.0 0.0 null null)
    (`KismetSystemLibrary.Delay` 0.2)
    (`self.K2_DestroyActor`)))

(event `self.ReceiveBeginPlay`
  (bind _asss_game_mode (cast `/Game/SpaceShooter/SS_GameMode` (`GameplayStatics.GetGameMode`)))
  (if (`/Game/SpaceShooter/SS_GameMode.TiempoRalentizado` _asss_game_mode)
    (set `self.CustomTimeDilation` 0.2)))

(event `self.ReceiveTick`
  (params (DeltaSeconds :type "Float (single-precision)"))
  (`self.K2_SetActorLocation` (+ (`self.K2_GetActorLocation`) (* (`self.GetActorForwardVector`) (* DeltaSeconds (`self.Speed`))))))

(fn `UserConstructionScript`)