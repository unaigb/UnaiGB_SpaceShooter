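; Player projectile actor for the space shooter that flies forward and damages enemies.
; Tick moves it along its forward vector at Speed without sweeping, so hits come from the Capsule's begin-overlap event.
; Overlaps branch on actor tags: enemies take fixed damage, SupInf actors just absorb the shot, and enemy ammo is destroyed along with it.
; The projectile destroys itself in all three cases.
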(event `self.Capsule.OnComponentBeginOverlap`
  (params (OverlappedComponent :type "PrimitiveComponent Object Reference") (OtherActor :type "Actor Object Reference") (OtherComp :type "PrimitiveComponent Object Reference") (OtherBodyIndex :type Integer) (bFromSweep :type Boolean) (SweepResult :type "HitResult Structure (by ref)"))
  (`/Engine/EditorBlueprintResources/StandardMacros.IsValid` OtherActor
    (:`Is Valid`
      (if (`self.ActorHasTag` OtherActor "Enemy")
        (`GameplayStatics.ApplyDamage` OtherActor 25.0)
        (`self.K2_DestroyActor`)
        (elif (`self.ActorHasTag` OtherActor "SupInf")
          (`self.K2_DestroyActor`)
          (elif (`self.ActorHasTag` OtherActor "EnemyAmmo")
            (`self.K2_DestroyActor` OtherActor)
            (`self.K2_DestroyActor`)))))))

(event `self.ReceiveTick`
  (params (DeltaSeconds :type "Float (single-precision)"))
  (`self.K2_SetActorLocation` (+ (`self.K2_GetActorLocation`) (* (`self.GetActorForwardVector`) (* DeltaSeconds (`self.Speed`))))))

(fn `UserConstructionScript`)